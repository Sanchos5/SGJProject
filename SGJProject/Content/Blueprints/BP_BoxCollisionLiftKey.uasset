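; BP_BoxCollisionLiftKey is a key-gated trigger that opens a pair of doors, apparently for a lift.
; When a BP_Player with IsKey set overlaps the Box, a DoOnce lets OpenDoor fire a single time.
; The DoorOpen timeline then drives LeftDoor and RightDoor along relative X through separate tracks, with no closing logic.
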(event `self.Box.OnComponentBeginOverlap`
  (params (OverlappedComponent :type "PrimitiveComponent Object Reference") (OtherActor :type "Actor Object Reference") (OtherComp :type "PrimitiveComponent Object Reference") (OtherBodyIndex :type Integer) (bFromSweep :type Boolean) (SweepResult :type "HitResult Structure (by ref)"))
  (bind _asbp_player (cast `/Game/Blueprints/BP_Player` OtherActor))
  (if (`/Game/Blueprints/BP_Player.IsKey?` _asbp_player)
    (`/Engine/EditorBlueprintResources/StandardMacros.DoOnce` false
      (:`Completed`
        (`self.OpenDoor`)))))

(event `OpenDoor`
  (bind _rightdoor (`self.RightDoor`))
  (bind _leftdoor (`self.LeftDoor`))
  (bind (_relativelocation_x _relativelocation_y _relativelocation_z) (`KismetMathLibrary.BreakVector` (`SceneComponent.RelativeLocation` _leftdoor)))
  (bind (_relativelocation_x_2 _relativelocation_y_2 _relativelocation_z_2) (`KismetMathLibrary.BreakVector` (`SceneComponent.RelativeLocation` _rightdoor)))
  (bind (_direction _left _right) (`Timeline|DoorOpen` :!via `PlayFromStart`)
    (:`Update`
      (`SceneComponent.K2_SetRelativeLocation` _leftdoor (`KismetMathLibrary.MakeVector` _left _relativelocation_y _relativelocation_z) false false)
      (`SceneComponent.K2_SetRelativeLocation` _rightdoor (`KismetMathLibrary.MakeVector` _right _relativelocation_y_2 _relativelocation_z_2) false false))))

(fn `UserConstructionScript`)