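; Weapon pickup actor that grants its WeaponClass to BP_Player when the player overlaps its sphere.
; Pickupitem sends the class to the player and destroys the pickup, then the overlap handler activates or deactivates the current weapon according to the battery component's GogglesEnabled state.
; Interact and Spin are empty; the looping line-trace timer and the hide and collision-disable nodes are unconnected.
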(event `self.Sphere.OnComponentBeginOverlap`
  (params (OverlappedComponent :type "PrimitiveComponent Object Reference") (OtherActor :type "Actor Object Reference") (OtherComp :type "PrimitiveComponent Object Reference") (OtherBodyIndex :type Integer) (bFromSweep :type Boolean) (SweepResult :type "HitResult Structure (by ref)"))
  (bind _asbp_player (cast `/Game/Blueprints/BP_Player` OtherActor))
  (bind _output_get (set `self.As BP Player` _asbp_player))
  (`self.Pickupitem` _output_get)
  (if (`BatteryComponent.bGogglesEnabled` (`BatteryComponent.FindBatteryComponent` _output_get))
    (bind _current_weapon (`/Game/Blueprints/BP_Player.Current Weapon` _output_get))
    (`/Game/Variant_Shooter/Blueprints/Pickups/BP_ShooterWeaponBase.Activate Weapon` _current_weapon)
    (else
      (`/Game/Variant_Shooter/Blueprints/Pickups/BP_ShooterWeaponBase.Deactivate Weapon` _current_weapon))))

(event `LineTraceEvent`
  (`/Game/Blueprints/BP_Player.Linetrace` (`self.As BP Player`)))

(event `self.Sphere.OnComponentEndOverlap`
  (params (OverlappedComponent :type "PrimitiveComponent Object Reference") (OtherActor :type "Actor Object Reference") (OtherComp :type "PrimitiveComponent Object Reference") (OtherBodyIndex :type Integer))
  (`KismetSystemLibrary.K2_ClearTimer` null "LineTraceEvent"))

(event `/Game/Blueprints/Pickups/BPI_Pickup.Interact`
  (params (OtherActor :type "Character Object Reference")))

(event `Pickupitem`
  (params (OtherActor :type "Character Object Reference"))
  (message `/Game/Variant_Shooter/Blueprints/Pickups/BPI_WeaponHolder.Add Weapon Class` OtherActor (`self.Weapon Class`))
  (`self.K2_DestroyActor`))

(fn `Spin`
  (params (`New Transform Scale` :type "Vector Structure")))

(fn `UserConstructionScript`)